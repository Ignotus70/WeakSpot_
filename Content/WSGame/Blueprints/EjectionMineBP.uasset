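; EjectionMineBP is a mine that, when activated, launches its projectile component and blows it up with visual effects.
; Activate reveals the projectile, and a timeline scales its Altura track by AlturaMaxProjectil to drive the relative Z position.
; When the timeline finishes, it spawns an explosion at the projectile and smoke at the exit point cached on BeginPlay, then destroys the projectile component.
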(event EventActivate
  (Rendering|SetVisibility (Variables|Default|GetMineProjectil) true false)
  (bind _altura (Timeline|ProjectilEjectionTL PlayFromStart)
    (:Update
      (Transformation|SetRelativeLocation (Variables|Default|GetMineProjectil) (Math|Vector|MakeVector 0.0 0.0 (* _altura (Variables|Default|GetAlturaMaxProjectil))) false false))
    (:Finished
      (Effects|SpawnEmitteratLocation "/Game/StarterContent/Particles/P_Explosion.P_Explosion" (Transformation|GetWorldLocation (Variables|Default|GetMineProjectil)))
      (Effects|SpawnEmitteratLocation "/Game/StarterContent/Particles/P_Smoke.P_Smoke" (Variables|Default|GetOriginProjectil))
      (Components|DestroyComponent (Variables|Default|GetMineProjectil)))))

(event EventBeginPlay
  ;[1 1 1] Captura posición original del proyectil (orificio de salida)
  (Variables|Default|SetOriginProjectil (Transformation|GetWorldLocation (Variables|Default|GetMineProjectil))))

(fn ConstructionScript
  (|CallParentFunction))